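; HorrorEngineCharacter is the player character for a horror game, handling movement, jumping, mouse look and a flashlight.
; Axis inputs move along the capsule's forward and right vectors, scaled by multipliers and frame delta time, while look input is scaled by mouse sensitivity.
; The flashlight input has two handlers: one toggles Flashlight visibility, the other attaches a new static mesh component to the right-hand socket on every press.
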(event Input|ActionEvents|InputAction[HE]Flashlight
  (params (Key :type Key%20Structure :default "None"))
  (:Pressed
    (bind _returnvalue (AddComponent|AddStaticMeshComponent false))
    (Transformation|AttachComponentToComponent _returnvalue (Variables|Character|GetMesh) "hand_rSocket" "SnapToTarget" "SnapToTarget" "SnapToTarget" true)))

(event Input|ActionEvents|InputAction[HE]Jump
  (params (Key :type Key%20Structure :default "None"))
  ;[0.498 0.6737 1] Jump Settings
  (:Pressed
    (Character|Jump))
  (:Released
    (Character|StopJumping)))

(event Input|ActionEvents|InputAction[HE]Flashlight
  (params (Key :type Key%20Structure :default "None"))
  (:Pressed
    (Rendering|SetVisibility (Variables|Default|GetFlashlight) (not (Rendering|IsVisible (Variables|Default|GetFlashlight))) false)))

(event Input|AxisEvents|InputAxis[HE]MoveForward
  (params (AxisValue :type Float%20%28single-precision%29))
  ;[0.498 0.6737 1] Movement
  (Pawn|Input|AddMovementInput (Math|Vector|GetForwardVector (Variables|Collision|GetCapsuleComponent)) (* AxisValue (Variables|Default|GetMovementMultipliers) (Utilities|Time|GetWorldDeltaSeconds)) false))

(event Input|AxisEvents|InputAxis[HE]MoveRight
  (params (AxisValue :type Float%20%28single-precision%29))
  ;[0.498 0.6737 1] Movement
  (Pawn|Input|AddMovementInput (Math|Vector|GetRightVector (Variables|Collision|GetCapsuleComponent)) (* AxisValue (Variables|Default|GetMovementMultipliers) (Utilities|Time|GetWorldDeltaSeconds)) false))

(event Input|AxisEvents|InputAxis[HE]LookUp
  (params (AxisValue :type Float%20%28single-precision%29))
  ;[0.498 0.6737 1] Movement
  (Pawn|Input|AddControllerPitchInput (* AxisValue (Variables|Default|GetMouseSensitivity))))

(event Input|AxisEvents|InputAxis[HE]Turn
  (params (AxisValue :type Float%20%28single-precision%29))
  ;[0.498 0.6737 1] Movement
  (Pawn|Input|AddControllerYawInput (* AxisValue (Variables|Default|GetMouseSensitivity))))

(fn ConstructionScript)